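; BP_ResourceMeter is an actor that runs a draining resource bar and triggers game over when it empties.
; BeginPlay creates the WBP_ResourceMeter widget, sets game-only input with mouse cursor and click events, and binds to the game instance's AddResource event.
; Tick drains the bar over time relative to the starting amount, AddResource events refill it, and at zero it stops ticking and broadcasts a "GameOver" notification.
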(event Custom|OnAddResource_Event_0
  (params (Amount :type Integer))
  (Progress|SetPercent (Variables|/Game/UI/WBP_ResourceMeter.WBP_ResourceMeter_C|GetResourceBar (stale EventBeginPlay _returnvalue_2)) (+ (Variables|/Script/UMG.ProgressBar|GetPercent (Variables|/Game/UI/WBP_ResourceMeter.WBP_ResourceMeter_C|GetResourceBar (stale EventBeginPlay _returnvalue_2))) (/ (Math|Conversions|ToFloat(Integer) Amount) (Variables|Default|GetResourcesAtStart)))))

(event EventBeginPlay
  (bind _returnvalue (Game|GetPlayerController 0))
  (bind _returnvalue_2 (UserInterface|CreateWidget "/Game/UI/WBP_ResourceMeter.WBP_ResourceMeter_C"))
  (UserInterface|Viewport|AddtoViewport _returnvalue_2 0)
  (Widget|SetVisibility _returnvalue_2 "Visible")
  (Variables|/Script/Engine.PlayerController|SetbEnableClickEvents _returnvalue true)
  (Input|SetInputModeGameOnly _returnvalue)
  (Variables|/Script/Engine.PlayerController|SetbShowMouseCursor _returnvalue true)
  (bind _aspcgame_instance (Utilities|Casting|CastToPCGameInstance (Game|GetGameInstance)))
  (EventDispatchers|AssignOnAddResource (Variables|/Script/PlasticCult.PCGameInstance|GetPCEvents _aspcgame_instance) (delegate Custom|OnAddResource_Event_0)))

(event Collision|EventActorBeginOverlap
  (params (OtherActor :type Actor%20Object%20Reference)))

(event EventTick
  (params (DeltaSeconds :type Float%20%28single-precision%29))
  (Progress|SetPercent (Variables|/Game/UI/WBP_ResourceMeter.WBP_ResourceMeter_C|GetResourceBar (stale EventBeginPlay _returnvalue_2)) (- (Variables|/Script/UMG.ProgressBar|GetPercent (Variables|/Game/UI/WBP_ResourceMeter.WBP_ResourceMeter_C|GetResourceBar (stale EventBeginPlay _returnvalue_2))) (* DeltaSeconds (/ (Variables|Default|GetResourcesDecrease) (Variables|Default|GetResourcesAtStart)))))
  (if (<= (Variables|/Script/UMG.ProgressBar|GetPercent (Variables|/Game/UI/WBP_ResourceMeter.WBP_ResourceMeter_C|GetResourceBar (stale EventBeginPlay _returnvalue_2))) 0.0)
    (Actor|Tick|SetActorTickEnabled false)
    (Default|CallOnNotificationHappens (Variables|/Script/PlasticCult.PCGameInstance|GetPCEvents (stale EventBeginPlay _aspcgame_instance)) "GameOver")))

(fn ConstructionScript)