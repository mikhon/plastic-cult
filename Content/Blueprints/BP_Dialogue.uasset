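; BP_Dialogue plays a scripted dialogue on screen at BeginPlay, then signals the game to start.
; It creates a WBP_Dialogue widget and types each Script1 line letter by letter through the WriteLine macro, a delayed character loop over growing substrings.
; After each line it pauses, clears the text and loops via EndOfLine.
; When the script ends, it fires a "StartGame" notification through PCGameInstance's PCEvents.
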(event Custom|EndOfLine
  (bind _script1 (Variables|Default|GetScript1))
  (bind _index (Variables|Default|GetIndex))
  ;[1 1 1] Write Script1 on the screen
  (if (< _index (Utilities|Array|Length _script1))
    (Utilities|WriteLine (stale EventBeginPlay _returnvalue) (Utilities|Array|Get(acopy) _script1 _index) 0.06
      (:Completed
        (Math|Integer|IncrementInt (Variables|Default|GetIndex)
          (:%20%20
            (Utilities|FlowControl|Delay 2.5)
            (Variables|/Game/UI/WBP_Dialogue.WBP_Dialogue_C|SetText (stale EventBeginPlay _returnvalue) "")
            (CallFunction|EndOfLine)))))
    (else
      (Default|CallOnNotificationHappens (Variables|/Script/PlasticCult.PCGameInstance|GetPCEvents (stale EventBeginPlay _aspcgame_instance)) "StartGame"))))

(event EventBeginPlay
  ;[1 1 1] Show Dialogue
  (bind _returnvalue (UserInterface|CreateWidget "/Game/UI/WBP_Dialogue.WBP_Dialogue_C"))
  (UserInterface|Viewport|AddtoViewport _returnvalue 2)
  (Widget|SetVisibility _returnvalue "Visible")
  ;[1 1 1] Get Global Events
  (bind _aspcgame_instance (Utilities|Casting|CastToPCGameInstance (Game|GetGameInstance)))
  ;[1 1 1] Write Script1 on the screen
  (Utilities|WriteLine _returnvalue (Utilities|Array|Get(acopy) (Variables|Default|GetScript1) (Variables|Default|GetIndex)) 0.06
    (:Completed
      (Math|Integer|IncrementInt (Variables|Default|GetIndex)
        (:%20%20
          (Utilities|FlowControl|Delay 2.5)
          (Variables|/Game/UI/WBP_Dialogue.WBP_Dialogue_C|SetText _returnvalue "")
          (CallFunction|EndOfLine))))))

(event Collision|EventActorBeginOverlap
  (params (OtherActor :type Actor%20Object%20Reference)))

(event EventTick
  (params (DeltaSeconds :type Float%20%28single-precision%29)))

(fn ConstructionScript)