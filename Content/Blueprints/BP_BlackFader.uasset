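; BP_BlackFader is an actor that drives a black screen fade through the WBP_BlackFader widget.
; On BeginPlay it binds to the game instance's PCEvents notification event, adds the widget to the viewport, and plays FadeOut after a fixed delay.
; Any notification other than "StartGame" plays FadeIn, then FadeOut after the same delay.
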(event Custom|NotificationHappens
  (params (NotificationId :type String))
  (if (Utilities|Enum|NotEqual(Enum) NotificationId "StartGame")
    (UserInterface|Animation|PlayAnimation (stale EventBeginPlay _returnvalue) (Variables|/Game/UI/WBP_BlackFader.WBP_BlackFader_C|GetFadeIn (stale EventBeginPlay _returnvalue)) 0.0 1 "Forward" 1.0 false)
    (Utilities|FlowControl|Delay 8.0)
    (UserInterface|Animation|PlayAnimation (stale EventBeginPlay _returnvalue) (Variables|/Game/UI/WBP_BlackFader.WBP_BlackFader_C|GetFadeOut (stale EventBeginPlay _returnvalue)) 0.0 1 "Forward" 1.0 false)))

(event EventBeginPlay
  ;[1 1 1] Get Global Events
  (bind _aspcgame_instance (Utilities|Casting|CastToPCGameInstance (Game|GetGameInstance)))
  (EventDispatchers|BindEventtoOnNotificationHappens (Variables|/Script/PlasticCult.PCGameInstance|GetPCEvents _aspcgame_instance) (delegate Custom|NotificationHappens))
  (bind _returnvalue (UserInterface|CreateWidget "/Game/UI/WBP_BlackFader.WBP_BlackFader_C"))
  (UserInterface|Viewport|AddtoViewport _returnvalue 1)
  (Widget|SetVisibility _returnvalue "Visible")
  (Utilities|FlowControl|Delay 8.0)
  (UserInterface|Animation|PlayAnimation _returnvalue (Variables|/Game/UI/WBP_BlackFader.WBP_BlackFader_C|GetFadeOut _returnvalue) 0.0 1 "Forward" 1.0 false))

(event Collision|EventActorBeginOverlap
  (params (OtherActor :type Actor%20Object%20Reference)))

(event EventTick
  (params (DeltaSeconds :type Float%20%28single-precision%29)))

(fn ConstructionScript)