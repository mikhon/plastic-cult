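; BP_Candelabra is a candelabra actor with logic to flicker its four point lights like candle flames.
; Each light has its own graph with a custom event that loops forever, waiting a short random delay and then setting a random intensity, so the lights vary independently.
; Nothing in this Blueprint calls those events, as BeginPlay, Tick and the construction script are empty.
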(event `self.ReceiveBeginPlay`)

(event `CustomEvent`
  (`KismetSystemLibrary.Delay` (`KismetMathLibrary.RandomFloatInRange` 0.0 0.2) :!label _label)
  (`LightComponent.SetIntensity` (`self.PointLight1`) (`KismetMathLibrary.RandomFloatInRange` 300.0 500.0))
  (goto _label))

(event `CustomEvent_1`
  (`KismetSystemLibrary.Delay` (`KismetMathLibrary.RandomFloatInRange` 0.0 0.2) :!label _label)
  (`LightComponent.SetIntensity` (`self.PointLight2`) (`KismetMathLibrary.RandomFloatInRange` 300.0 500.0))
  (goto _label))

(event `CustomEvent_2`
  (`KismetSystemLibrary.Delay` (`KismetMathLibrary.RandomFloatInRange` 0.0 0.2) :!label _label)
  (`LightComponent.SetIntensity` (`self.PointLight4`) (`KismetMathLibrary.RandomFloatInRange` 300.0 500.0))
  (goto _label))

(event `CustomEvent_3`
  (`KismetSystemLibrary.Delay` (`KismetMathLibrary.RandomFloatInRange` 0.0 0.2) :!label _label)
  (`LightComponent.SetIntensity` (`self.PointLight`) (`KismetMathLibrary.RandomFloatInRange` 300.0 500.0))
  (goto _label))

(fn `UserConstructionScript`)